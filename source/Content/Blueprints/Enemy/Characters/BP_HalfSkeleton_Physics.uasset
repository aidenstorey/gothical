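; BP_HalfSkeleton_Physics is an enemy half-skeleton physics prop that is knocked by an impulse when it spawns and later dissolves.
; On BeginPlay it creates a dynamic instance of the mesh's first material and applies a randomized radial velocity impulse near the actor's origin.
; After a short delay, a timeline drives the DissolveAmount parameter on that material.
; The graph never destroys the actor.
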(event EventBeginPlay
  (bind _skeletalmeshcomponent (Variables|SkeletalMeshActor|GetSkeletalMeshComponent))
  (bind _returnvalue (Rendering|Material|CreateDynamicMaterialInstance _skeletalmeshcomponent 0 (Rendering|Material|GetMaterial _skeletalmeshcomponent 0) :!class /Script/Engine.PrimitiveComponent))
  (Utilities|Array|Add (Variables|Default|GetDissolveMaterial) _returnvalue)
  (Physics|AddRadialImpulse (Variables|SkeletalMeshActor|GetSkeletalMeshComponent) (+ (Transformation|GetActorLocation) (* (Math|Random|RandomUnitVector) (Math|Random|RandomFloatinRange 0.0 1e+01))) 1e+02 (Math|Random|RandomFloatinRange 5e+02 4e+02) "RIF_Constant" true)
  (Utilities|FlowControl|Delay 0 3.0)
  (bind _dissolve (Timeline|Timeline_0 Play)
    (:Update
      (for _array_element (Variables|Default|GetDissolveMaterial)
        (Rendering|Material|SetScalarParameterValue _array_element "DissolveAmount" _dissolve :!class /Script/Engine.MaterialInstanceDynamic)))))

(fn ConstructionScript)