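; Cathedral Guardian boss character that translates boss states into animation and HUD feedback.
; OnStateChange sets Reap, Rend, Harvest and hit flags on the AnimBlueprint, spawns the Harvest particle, and binds and shows the HUD health bar on Seeking.
; Damage indicators also put the boss controller into its hit state, and destruction hides the bar and ends boss music.
; Undissolve reverses a dissolve timeline across two dynamic materials created in the construction script.
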(event Custom|Undissolve
  (bind _dissolveamount (Timeline|Dissolve ReverseFromEnd)
    (:Update
      (for _array_element (Variables|Default|GetDynamicMaterial)
        (Rendering|Material|SetScalarParameterValue _array_element "DissolveAmount" _dissolveamount :!class /Script/Engine.MaterialInstanceDynamic)))))

(event EventDestroyed
  (bind _ascontroller_player (Utilities|Casting|CastToControllerPlayer (Game|GetPlayerController 0)))
  (bind _returnvalue (Class|ControllerPlayer|GetCurrentWidget _ascontroller_player))
  (bind _asbp_hud (Utilities|Casting|CastToBP_HUD _returnvalue))
  (Widget|SetVisibility (Variables|/Game/HUD/BP_HUD.BP_HUD_C|Getboss_health_bar _asbp_hud) "Hidden")
  (Default|EndBossMusic (Variables|Default|GetAudioController)))

(event EventSpawnIndicator
  (params (_krfDamageAmount :type Float%20%28single-precision%29%20%28by%20ref%29))
  (|CallParentFunction _krfDamageAmount)
  (bind _returnvalue (AI|GetAIController self))
  (bind _asboss_controller_base (Utilities|Casting|CastToBossControllerBase _returnvalue))
  (Class|BossControllerBase|EnterHitState _asboss_controller_base 1.0))

(fn ConstructionScript
  (bind _mesh (Variables|Character|GetMesh))
  (bind _mesh_2 (Variables|Character|GetMesh))
  (bind _returnvalue (Rendering|Material|CreateDynamicMaterialInstance _mesh_2 0 (Rendering|Material|GetMaterial _mesh_2 0) :!class /Script/Engine.PrimitiveComponent))
  (Utilities|Array|Add (Variables|Default|GetDynamicMaterial) _returnvalue)
  (bind _returnvalue_2 (Rendering|Material|CreateDynamicMaterialInstance _mesh 1 (Rendering|Material|GetMaterial _mesh 1) :!class /Script/Engine.PrimitiveComponent))
  (Utilities|Array|Add (Variables|Default|GetDynamicMaterial) _returnvalue_2))

(fn OnStateChange
  (params (NewState :type EBossState%20Enum))
  (bind _asbp_cathedral_guardian_anim_blueprint (Utilities|Casting|CastToBP_CathedralGuardian_AnimBlueprint (Components|SkeletalMesh|GetAnimInstance (Variables|Character|GetMesh))))
  (switch Utilities|FlowControl|Switch|SwitchonEBossState NewState
    (:BOSS_STATE_IDLE
      (Variables|/Game/Animations/Enemies/Bosses/CathedralGuardian/BP_CathedralGuardian_AnimBlueprint.BP_CathedralGuardian_AnimBlueprint_C|SetReap _asbp_cathedral_guardian_anim_blueprint false :!label _label)
      (Variables|/Game/Animations/Enemies/Bosses/CathedralGuardian/BP_CathedralGuardian_AnimBlueprint.BP_CathedralGuardian_AnimBlueprint_C|SetRend _asbp_cathedral_guardian_anim_blueprint false)
      (Variables|/Game/Animations/Enemies/Bosses/CathedralGuardian/BP_CathedralGuardian_AnimBlueprint.BP_CathedralGuardian_AnimBlueprint_C|SetHarvest _asbp_cathedral_guardian_anim_blueprint false))
    (:BOSS_STATE_SEEKING
      (bind _ascontroller_player (Utilities|Casting|CastToControllerPlayer (Game|GetPlayerController 0)))
      (bind _returnvalue (Class|ControllerPlayer|GetCurrentWidget _ascontroller_player))
      (bind _asbp_hud (Utilities|Casting|CastToBP_HUD _returnvalue))
      (Variables|/Game/HUD/BP_HUD.BP_HUD_C|SetCurrentBoss _asbp_hud (Pawn|GetController self))
      (Widget|SetVisibility (Variables|/Game/HUD/BP_HUD.BP_HUD_C|Getboss_health_bar _asbp_hud) "Visible")
      (goto _label))
    (:BOSS_STATE_PRE_ATTACK_A
      (Variables|/Game/Animations/Enemies/Bosses/CathedralGuardian/BP_CathedralGuardian_AnimBlueprint.BP_CathedralGuardian_AnimBlueprint_C|SetReap _asbp_cathedral_guardian_anim_blueprint true))
    (:BOSS_STATE_PRE_ATTACK_B
      (Variables|/Game/Animations/Enemies/Bosses/CathedralGuardian/BP_CathedralGuardian_AnimBlueprint.BP_CathedralGuardian_AnimBlueprint_C|SetRend _asbp_cathedral_guardian_anim_blueprint true))
    (:BOSS_STATE_PRE_ATTACK_C
      (Variables|/Game/Animations/Enemies/Bosses/CathedralGuardian/BP_CathedralGuardian_AnimBlueprint.BP_CathedralGuardian_AnimBlueprint_C|SetHarvest _asbp_cathedral_guardian_anim_blueprint true)
      (Effects|SpawnEmitteratLocation "/Game/VFX/P_CathedralGuardianHarvest.P_CathedralGuardianHarvest" (- (Transformation|GetActorLocation) "0, 0,140.000000")))
    (:BOSS_STATE_PRE_HIT
      (Variables|/Game/Animations/Enemies/Bosses/CathedralGuardian/BP_CathedralGuardian_AnimBlueprint.BP_CathedralGuardian_AnimBlueprint_C|SetIsHit _asbp_cathedral_guardian_anim_blueprint true)
      (Variables|/Game/Animations/Enemies/Bosses/CathedralGuardian/BP_CathedralGuardian_AnimBlueprint.BP_CathedralGuardian_AnimBlueprint_C|SetReap _asbp_cathedral_guardian_anim_blueprint false)
      (Variables|/Game/Animations/Enemies/Bosses/CathedralGuardian/BP_CathedralGuardian_AnimBlueprint.BP_CathedralGuardian_AnimBlueprint_C|SetRend _asbp_cathedral_guardian_anim_blueprint false)
      (Variables|/Game/Animations/Enemies/Bosses/CathedralGuardian/BP_CathedralGuardian_AnimBlueprint.BP_CathedralGuardian_AnimBlueprint_C|SetHarvest _asbp_cathedral_guardian_anim_blueprint false))
    (:BOSS_STATE_POST_HIT
      (Variables|/Game/Animations/Enemies/Bosses/CathedralGuardian/BP_CathedralGuardian_AnimBlueprint.BP_CathedralGuardian_AnimBlueprint_C|SetIsHit _asbp_cathedral_guardian_anim_blueprint false))))