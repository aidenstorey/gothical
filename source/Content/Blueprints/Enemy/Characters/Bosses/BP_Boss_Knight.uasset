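; Knight boss character with a stomp attack that shakes the camera and a telegraphed high-speed charge.
; OnStateChange maps boss states to anim blueprint flags, movement speed and the HUD boss health bar.
; While charging, box overlaps launch and damage characters and cancel the charge, while other obstacles put the controller into a hit state, as does SpawnIndicator.
; Destruction spawns a physics corpse, plays a death sound, hides the bar and ends boss music.
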(event OnComponentBeginOverlap(Box)
  (params (OtherActor :type Actor%20Object%20Reference) (OtherComp :type Primitive%20Component%20Object%20Reference) (OtherBodyIndex :type Integer) (bFromSweep :type Boolean) (SweepResult :type Hit%20Result%20Structure%20%28by%20ref%29))
  (if (Variables|Default|GetCharging)
    (bind _ascharacter (Utilities|Casting|CastToCharacter OtherActor)
      (:then
        (Physics|AddImpulse (Variables|/Script/Engine.Character|GetCharacterMovement _ascharacter) (* (+ (Math|Vector|Normalize (- (Transformation|GetActorLocation OtherActor) (Transformation|GetActorLocation self))) "0, 0,0.700000") 1e+03) true)
        (Game|Damage|ApplyDamage OtherActor 1e+01 0 self "/Script/Engine.DamageType")
        (bind _returnvalue (AI|GetAIController self))
        (bind _asboss_knight_controller (Utilities|Casting|CastToBossKnightController _returnvalue))
        (Class|BossKnightController|CancelCharge _asboss_knight_controller))
      (:CastFailed
        (bind _returnvalue_2 (AI|GetAIController self))
        (bind _asboss_knight_controller_2 (Utilities|Casting|CastToBossKnightController _returnvalue_2))
        (Class|BossControllerBase|EnterHitState _asboss_knight_controller_2 1.0)))))

(event EventDestroyed
  (bind _returnvalue (Transformation|GetActorLocation))
  (Audio|PlaySoundatLocation 0 "/Game/Sound/SoundWaves/Enemies/Bosses/Knight/Knight_Death.Knight_Death" _returnvalue)
  (Game|SpawnActorfromClass "/Game/Blueprints/Enemy/Characters/Bosses/BP_Knight_Physics_Final.BP_Knight_Physics_Final_C" (Math|Transform|MakeTransform (- _returnvalue "0, 0,90.000000") (Class|KismetMathLibrary|MakeRot 0.0 (.Yaw (Class|KismetMathLibrary|BreakRot (Transformation|GetWorldRotation (Variables|Character|GetMesh)))) 2.7e+02) "1,1,1") true 0 0)
  (bind _ascontroller_player (Utilities|Casting|CastToControllerPlayer (Game|GetPlayerController 0)))
  (bind _returnvalue_2 (Class|ControllerPlayer|GetCurrentWidget _ascontroller_player))
  (bind _asbp_hud (Utilities|Casting|CastToBP_HUD _returnvalue_2))
  (Widget|SetVisibility (Variables|/Game/HUD/BP_HUD.BP_HUD_C|Getboss_health_bar _asbp_hud) "Hidden")
  (Default|EndBossMusic (Variables|Default|GetAudioController)))

(event EventBeginPlay
  (Variables|/Script/Engine.CharacterMovementComponent|SetMaxWalkSpeed (Variables|Character|GetCharacterMovement self) 2e+02)
  (|CallParentFunction))

(event EventSpawnIndicator
  (params (_krfDamageAmount :type Float%20%28single-precision%29%20%28by%20ref%29))
  (|CallParentFunction _krfDamageAmount)
  (bind _returnvalue (AI|GetAIController self))
  (bind _asboss_controller_base (Utilities|Casting|CastToBossControllerBase _returnvalue))
  (Class|BossControllerBase|EnterHitState _asboss_controller_base 1.0))

(fn ConstructionScript)

(fn OnStateChange
  (params (BossState :type Byte))
  (bind _charactermovement (Variables|Character|GetCharacterMovement))
  (bind _asbp_boss_knight_anim_blueprint (Utilities|Casting|CastToBP_BossKnight_AnimBlueprint (Components|SkeletalMesh|GetAnimInstance (Variables|Character|GetMesh))))
  (switch Utilities|FlowControl|Switch|SwitchonEBossState BossState
    (:BOSS_STATE_IDLE
      (Variables|/Game/Animations/Enemies/Bosses/Knight/BP_BossKnight_AnimBlueprint.BP_BossKnight_AnimBlueprint_C|SetIsWalking _asbp_boss_knight_anim_blueprint false)
      (Variables|/Game/Animations/Enemies/Bosses/Knight/BP_BossKnight_AnimBlueprint.BP_BossKnight_AnimBlueprint_C|SetIsStomping _asbp_boss_knight_anim_blueprint false))
    (:BOSS_STATE_SEEKING
      (Variables|/Game/Animations/Enemies/Bosses/Knight/BP_BossKnight_AnimBlueprint.BP_BossKnight_AnimBlueprint_C|SetIsWalking _asbp_boss_knight_anim_blueprint true)
      (Variables|/Game/Animations/Enemies/Bosses/Knight/BP_BossKnight_AnimBlueprint.BP_BossKnight_AnimBlueprint_C|SetIsStomping _asbp_boss_knight_anim_blueprint false)
      (bind _ascontroller_player (Utilities|Casting|CastToControllerPlayer (Game|GetPlayerController 0)))
      (bind _returnvalue (Class|ControllerPlayer|GetCurrentWidget _ascontroller_player))
      (bind _asbp_hud (Utilities|Casting|CastToBP_HUD _returnvalue))
      (Variables|/Game/HUD/BP_HUD.BP_HUD_C|SetCurrentBoss _asbp_hud (Pawn|GetController self))
      (Widget|SetVisibility (Variables|/Game/HUD/BP_HUD.BP_HUD_C|Getboss_health_bar _asbp_hud) "Visible"))
    (:BOSS_STATE_PRE_ATTACK_A
      (Variables|/Game/Animations/Enemies/Bosses/Knight/BP_BossKnight_AnimBlueprint.BP_BossKnight_AnimBlueprint_C|SetIsWalking _asbp_boss_knight_anim_blueprint false)
      (Variables|/Game/Animations/Enemies/Bosses/Knight/BP_BossKnight_AnimBlueprint.BP_BossKnight_AnimBlueprint_C|SetIsStomping _asbp_boss_knight_anim_blueprint true)
      (Components|Movement|StopMovementImmediately (Variables|Character|GetCharacterMovement) :!label _label))
    (:BOSS_STATE_ATTACK_A
      (Class|PlayerController|ClientPlayCameraShake (Game|GetPlayerController 0) "/Game/Blueprints/BP_Camera_Shake.BP_Camera_Shake_C" 2e+01 "CameraLocal" "0, 0, 0"))
    (:BOSS_STATE_PRE_ATTACK_B
      (Variables|/Game/Animations/Enemies/Bosses/Knight/BP_BossKnight_AnimBlueprint.BP_BossKnight_AnimBlueprint_C|SetIsWalking _asbp_boss_knight_anim_blueprint false)
      (Variables|/Game/Animations/Enemies/Bosses/Knight/BP_BossKnight_AnimBlueprint.BP_BossKnight_AnimBlueprint_C|SetIsTaunting _asbp_boss_knight_anim_blueprint true)
      (goto _label))
    (:BOSS_STATE_ATTACK_B
      (Variables|/Game/Animations/Enemies/Bosses/Knight/BP_BossKnight_AnimBlueprint.BP_BossKnight_AnimBlueprint_C|SetIsCharging _asbp_boss_knight_anim_blueprint true)
      (Variables|Default|SetCharging true)
      (Variables|/Script/Engine.CharacterMovementComponent|SetMaxWalkSpeed _charactermovement 1e+03)
      (Variables|/Script/Engine.CharacterMovementComponent|SetMaxAcceleration _charactermovement 1e+04))
    (:BOSS_STATE_POST_ATTACK_B
      (Variables|/Game/Animations/Enemies/Bosses/Knight/BP_BossKnight_AnimBlueprint.BP_BossKnight_AnimBlueprint_C|SetIsCharging _asbp_boss_knight_anim_blueprint false)
      (Variables|/Game/Animations/Enemies/Bosses/Knight/BP_BossKnight_AnimBlueprint.BP_BossKnight_AnimBlueprint_C|SetIsTaunting _asbp_boss_knight_anim_blueprint false)
      (Variables|Default|SetCharging false)
      (Variables|/Script/Engine.CharacterMovementComponent|SetMaxWalkSpeed (Variables|Character|GetCharacterMovement) 1.8e+02))
    (:BOSS_STATE_PRE_HIT
      (Variables|/Game/Animations/Enemies/Bosses/Knight/BP_BossKnight_AnimBlueprint.BP_BossKnight_AnimBlueprint_C|SetIsHit _asbp_boss_knight_anim_blueprint true)
      (Variables|/Game/Animations/Enemies/Bosses/Knight/BP_BossKnight_AnimBlueprint.BP_BossKnight_AnimBlueprint_C|SetIsCharging _asbp_boss_knight_anim_blueprint false)
      (Variables|/Game/Animations/Enemies/Bosses/Knight/BP_BossKnight_AnimBlueprint.BP_BossKnight_AnimBlueprint_C|SetIsTaunting _asbp_boss_knight_anim_blueprint false)
      (Variables|Default|SetCharging false)
      (Variables|/Game/Animations/Enemies/Bosses/Knight/BP_BossKnight_AnimBlueprint.BP_BossKnight_AnimBlueprint_C|SetIsWalking _asbp_boss_knight_anim_blueprint false)
      (Variables|/Game/Animations/Enemies/Bosses/Knight/BP_BossKnight_AnimBlueprint.BP_BossKnight_AnimBlueprint_C|SetIsStomping _asbp_boss_knight_anim_blueprint false)
      (Variables|/Script/Engine.CharacterMovementComponent|SetMaxWalkSpeed (Variables|Character|GetCharacterMovement) 1.8e+02))
    (:BOSS_STATE_POST_HIT
      (Variables|/Game/Animations/Enemies/Bosses/Knight/BP_BossKnight_AnimBlueprint.BP_BossKnight_AnimBlueprint_C|SetIsHit _asbp_boss_knight_anim_blueprint false))))