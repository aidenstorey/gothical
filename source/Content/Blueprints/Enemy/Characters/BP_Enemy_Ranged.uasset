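; Ranged enemy character, a bat, that links its state changes to animation and sound.
; OnStateChange sets IsAttacking on the bat AnimBlueprint, clearing it in Idle and setting it in Pre Attack and Post Attack.
; Post Attack also plays the attack sound at the actor's location, and destruction of the actor plays a death sound.
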(event EventDestroyed
  (Audio|PlaySoundatLocation 0 "/Game/Sound/SoundWaves/Enemies/Bat_Death.Bat_Death" (Transformation|GetActorLocation self) 0.7))

(fn ConstructionScript)

(fn OnStateChange
  (params (NewParam :type EEnemyState%20Enum))
  (bind _asbp_bat_new_anim_blueprint (Utilities|Casting|CastToBP_bat_new_AnimBlueprint (Components|SkeletalMesh|GetAnimInstance (Variables|Character|GetMesh self))))
  (switch Utilities|FlowControl|Switch|SwitchonEEnemyState NewParam
    (:ENEMY_STATE_IDLE
      (Variables|/Game/Animations/Enemies/Mobs/Flying/Bat/BP_bat_new_AnimBlueprint.BP_bat_new_AnimBlueprint_C|Setis_attacking _asbp_bat_new_anim_blueprint false))
    (:ENEMY_STATE_PRE_ATTACK
      (Variables|/Game/Animations/Enemies/Mobs/Flying/Bat/BP_bat_new_AnimBlueprint.BP_bat_new_AnimBlueprint_C|Setis_attacking _asbp_bat_new_anim_blueprint true :!label _label))
    (:ENEMY_STATE_POST_ATTACK
      (Audio|PlaySoundatLocation 0 "/Game/Sound/SoundWaves/Enemies/Bat_Attack.Bat_Attack" (Transformation|GetActorLocation self))
      (goto _label))))