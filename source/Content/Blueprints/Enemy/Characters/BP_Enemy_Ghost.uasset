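; BP_Enemy_Ghost is a ghost enemy character that reacts to AI state changes and deals contact damage while attacking.
; ChangeState drives the ghost AnimBP's IsAttacking flag and walk speed, speeding up in Pre Attack and resetting in Idle or Post Attack, with an occasional random noise when Seeking.
; Capsule overlaps during an attack apply damage taken from the EnemyControllerBase characteristics, using the AnimBP flag as the gate.
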(event OnComponentBeginOverlap(CapsuleComponent)
  (params (OtherActor :type Actor%20Object%20Reference) (OtherComp :type Primitive%20Component%20Object%20Reference) (OtherBodyIndex :type Integer) (bFromSweep :type Boolean) (SweepResult :type Hit%20Result%20Structure%20%28by%20ref%29))
  (bind _asbp_ghost_anim_blueprint (Utilities|Casting|CastToBP_ghost_AnimBlueprint (Components|SkeletalMesh|GetAnimInstance (Variables|Character|GetMesh))))
  (if (Variables|/Game/Animations/Enemies/Mobs/Flying/Ghost/BP_ghost_AnimBlueprint.BP_ghost_AnimBlueprint_C|Getis_attacking _asbp_ghost_anim_blueprint)
    (bind _returnvalue (AI|GetAIController self))
    (bind _asenemy_controller_base (Utilities|Casting|CastToEnemyControllerBase _returnvalue))
    (bind _returnvalue_2 (Class|EnemyControllerBase|GetCharacteristics _asenemy_controller_base))
    (Game|Damage|ApplyDamage OtherActor (Math|Conversions|ToFloat(Integer) (Class|Characteristics|GetDamage _returnvalue_2)) (Pawn|GetController) self "/Script/Engine.DamageType")))

(event EventBeginPlay
  (|CallParentFunction))

(event EventChangeState
  (params (New%20State :type EEnemyState%20Enum :default "ENEMY_STATE_IDLE"))
  (bind _charactermovement (Variables|Character|GetCharacterMovement))
  (bind _asbp_ghost_anim_blueprint (Utilities|Casting|CastToBP_ghost_AnimBlueprint (Components|SkeletalMesh|GetAnimInstance (Variables|Character|GetMesh))))
  (switch Utilities|FlowControl|Switch|SwitchonEEnemyState New%20State
    (:ENEMY_STATE_IDLE
      (Variables|/Game/Animations/Enemies/Mobs/Flying/Ghost/BP_ghost_AnimBlueprint.BP_ghost_AnimBlueprint_C|Setis_attacking _asbp_ghost_anim_blueprint false :!label _label)
      (Variables|/Script/Engine.CharacterMovementComponent|SetMaxWalkSpeed _charactermovement 3.5e+02))
    (:ENEMY_STATE_SEEKING
      (if (== (Math|Random|RandomIntegerinRange 0 8) 0)
        (Audio|PlaySoundatLocation "/Game/Sound/SoundCues/GhostNoise.GhostNoise" (Transformation|GetActorLocation self))))
    (:ENEMY_STATE_PRE_ATTACK
      (Variables|/Game/Animations/Enemies/Mobs/Flying/Ghost/BP_ghost_AnimBlueprint.BP_ghost_AnimBlueprint_C|Setis_attacking _asbp_ghost_anim_blueprint true)
      (Variables|/Script/Engine.CharacterMovementComponent|SetMaxWalkSpeed _charactermovement 5e+02))
    (:ENEMY_STATE_POST_ATTACK
      (goto _label))))

(fn ConstructionScript
  (|CallParentFunction))