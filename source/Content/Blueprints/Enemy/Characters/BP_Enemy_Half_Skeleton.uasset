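; Half-skeleton enemy character that links hit reactions, animation and death effects to its AI state.
; Its damage-indicator event puts the half-skeleton AI controller into a brief hit state before calling the parent's indicator logic.
; State changes set the attacking and hit flags on the Anim Blueprint.
; On destruction it plays a death sound and spawns a physics skeleton actor, lowered and rolled to lie at the mesh's yaw.
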(event EventChangeState
  (params (NewState :type Byte :default 0))
  (bind _asbp_half_skeleton_anim (Utilities|Casting|CastToBP_HalfSkeleton_Anim (Components|SkeletalMesh|GetAnimInstance (Variables|Character|GetMesh self))))
  (switch Utilities|FlowControl|Switch|SwitchonEEnemyState NewState
    (:ENEMY_STATE_IDLE
      (Variables|/Game/Animations/Enemies/Mobs/Melee/HalfSkeleton/BP_HalfSkeleton_Anim.BP_HalfSkeleton_Anim_C|SetIsAttacking _asbp_half_skeleton_anim false :!label _label)
      (Variables|/Game/Animations/Enemies/Mobs/Melee/HalfSkeleton/BP_HalfSkeleton_Anim.BP_HalfSkeleton_Anim_C|SetIsHit _asbp_half_skeleton_anim false :!label _label_2))
    (:ENEMY_STATE_SEEKING
      (goto _label))
    (:ENEMY_STATE_FLEEING
      (goto _label))
    (:ENEMY_STATE_PRE_ATTACK
      (Variables|/Game/Animations/Enemies/Mobs/Melee/HalfSkeleton/BP_HalfSkeleton_Anim.BP_HalfSkeleton_Anim_C|SetIsAttacking _asbp_half_skeleton_anim true)
      (goto _label_2))
    (:ENEMY_STATE_PRE_HIT
      (Variables|/Game/Animations/Enemies/Mobs/Melee/HalfSkeleton/BP_HalfSkeleton_Anim.BP_HalfSkeleton_Anim_C|SetIsHit _asbp_half_skeleton_anim true))
    (:ENEMY_STATE_POST_HIT
      (Variables|/Game/Animations/Enemies/Mobs/Melee/HalfSkeleton/BP_HalfSkeleton_Anim.BP_HalfSkeleton_Anim_C|SetIsHit _asbp_half_skeleton_anim false))))

(event EventSpawnIndicator
  (params (_krfDamageAmount :type Float%20%28single-precision%29%20%28by%20ref%29))
  (bind _returnvalue (AI|GetAIController self))
  (bind _asbp_enemy_controller_half_skeleton (Utilities|Casting|CastToBP_Enemy_Controller_Half_Skeleton _returnvalue))
  (Class|EnemyControllerBase|EnterHitState _asbp_enemy_controller_half_skeleton 0.49)
  (|CallParentFunction _krfDamageAmount))

(event EventDestroyed
  (Audio|PlaySoundatLocation 0 "/Game/Sound/SoundWaves/Enemies/Enemy_Skeleton_Death.Enemy_Skeleton_Death" (Transformation|GetActorLocation self) 0.1)
  (Game|SpawnActorfromClass "/Game/Blueprints/Enemy/Characters/BP_HalfSkeleton_Physics.BP_HalfSkeleton_Physics_C" (Math|Transform|MakeTransform (- (Transformation|GetActorLocation) "0, 0,90.000000") (Class|KismetMathLibrary|MakeRot 0.0 (.Yaw (Class|KismetMathLibrary|BreakRot (Transformation|GetWorldRotation (Variables|Character|GetMesh)))) 2.7e+02) "1,1,1") false 0 0))

(fn ConstructionScript
  (|CallParentFunction))