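; Melee skeleton enemy character that handles hit reactions, animation state and death remains.
; Spawning a damage indicator first puts its melee AI controller into a timed hit state, then runs the parent logic.
; ChangeState maps AI states onto attack and hit flags in the skeleton AnimBlueprint.
; On destruction it plays a death sound and spawns a physics skeleton, or one time in five a half-skeleton enemy plus discarded physics bones.
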(event EventBeginPlay
  (|CallParentFunction))

(event EventDestroyed
  (bind _returnvalue (Transformation|GetActorLocation))
  (bind _mesh (Variables|Character|GetMesh))
  (bind _returnvalue_2 (Transformation|GetWorldRotation _mesh))
  (bind _returnvalue_3 (- _returnvalue "0, 0,90.000000"))
  (bind _yaw (Class|KismetMathLibrary|BreakRot _returnvalue_2))
  (bind _returnvalue_4 (Class|KismetMathLibrary|MakeRot 0.0 _yaw 2.7e+02))
  (Audio|PlaySoundatLocation 0 "/Game/Sound/SoundWaves/Enemies/Enemy_Skeleton_Death.Enemy_Skeleton_Death" (Transformation|GetActorLocation self) 0.1)
  (if (== (Math|Random|RandomIntegerinRange 0 4) 0)
    (Game|SpawnActorfromClass "/Game/Blueprints/Enemy/Characters/BP_Enemy_Half_Skeleton.BP_Enemy_Half_Skeleton_C" (Math|Transform|MakeTransform _returnvalue_3 _returnvalue_2 "1,1,1") true 0 0)
    (Game|SpawnActorfromClass "/Game/Blueprints/Enemy/Characters/BP_SkeletonDiscard_Physics.BP_SkeletonDiscard_Physics_C" (Math|Transform|MakeTransform _returnvalue_3 _returnvalue_4 "1,1,1") false 0 0)
    (else
      (Game|SpawnActorfromClass "/Game/Blueprints/Enemy/Characters/BP_Skeleton_Physics.BP_Skeleton_Physics_C" (Math|Transform|MakeTransform _returnvalue_3 _returnvalue_4 "1,1,1") true 0 0))))

(event EventSpawnIndicator
  (params (_krfDamageAmount :type Float%20%28single-precision%29%20%28by%20ref%29))
  (bind _returnvalue (AI|GetAIController self))
  (bind _asbp_enemy_controller_melee (Utilities|Casting|CastToBP_Enemy_Controller_Melee _returnvalue))
  (Class|EnemyControllerBase|EnterHitState _asbp_enemy_controller_melee 0.95)
  (|CallParentFunction _krfDamageAmount))

(fn ConstructionScript)

(fn ChangeState
  (params (NewState :type Byte))
  (bind _asbp_enemy_skeleton_melee_anim_blueprint (Utilities|Casting|CastToBP_EnemySkeletonMelee_AnimBlueprint (Components|SkeletalMesh|GetAnimInstance (Variables|Character|GetMesh self))))
  (switch Utilities|FlowControl|Switch|SwitchonEEnemyState NewState
    (:ENEMY_STATE_IDLE
      (Variables|/Game/Animations/Enemies/Mobs/Melee/AxeSkeleton/BP_EnemySkeletonMelee_AnimBlueprint.BP_EnemySkeletonMelee_AnimBlueprint_C|SetIsAttacking _asbp_enemy_skeleton_melee_anim_blueprint false)
      (Variables|/Game/Animations/Enemies/Mobs/Melee/AxeSkeleton/BP_EnemySkeletonMelee_AnimBlueprint.BP_EnemySkeletonMelee_AnimBlueprint_C|SetIsHit _asbp_enemy_skeleton_melee_anim_blueprint false :!label _label))
    (:ENEMY_STATE_SEEKING
      (Variables|/Game/Animations/Enemies/Mobs/Melee/AxeSkeleton/BP_EnemySkeletonMelee_AnimBlueprint.BP_EnemySkeletonMelee_AnimBlueprint_C|SetIsAttacking _asbp_enemy_skeleton_melee_anim_blueprint false :!label _label_2)
      (goto _label))
    (:ENEMY_STATE_FLEEING
      (goto _label_2))
    (:ENEMY_STATE_PRE_ATTACK
      (Variables|/Game/Animations/Enemies/Mobs/Melee/AxeSkeleton/BP_EnemySkeletonMelee_AnimBlueprint.BP_EnemySkeletonMelee_AnimBlueprint_C|SetIsAttacking _asbp_enemy_skeleton_melee_anim_blueprint true)
      (goto _label))
    (:ENEMY_STATE_PRE_HIT
      (Variables|/Game/Animations/Enemies/Mobs/Melee/AxeSkeleton/BP_EnemySkeletonMelee_AnimBlueprint.BP_EnemySkeletonMelee_AnimBlueprint_C|SetIsHit _asbp_enemy_skeleton_melee_anim_blueprint true))
    (:ENEMY_STATE_POST_HIT
      (Variables|/Game/Animations/Enemies/Mobs/Melee/AxeSkeleton/BP_EnemySkeletonMelee_AnimBlueprint.BP_EnemySkeletonMelee_AnimBlueprint_C|SetIsHit _asbp_enemy_skeleton_melee_anim_blueprint false))))