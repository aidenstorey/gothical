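; Base enemy character Blueprint that handles visual feedback for hits, poison, freeze and damage taken.
; Status events edit channels of a dynamic material's TintValue: red for hits, green poison, blue freeze, with timelines on hit and effect end.
; SpawnIndicator shows a damage number widget at the enemy's projected screen position.
; BeginPlay creates the material instance and briefly freezes animation for a random delay, staggering playback between enemies.
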(event EventStartFreeze
  (bind _dynamic_material (Variables|Default|GetDynamic%20Material))
  (bind _returnvalue (Rendering|Material|GetVectorParameterValue _dynamic_material "TintValue" :!class /Script/Engine.MaterialInstanceDynamic))
  (Rendering|Material|SetVectorParameterValue _dynamic_material "TintValue" (Utilities|Struct|MakeLinearColor (.R (Utilities|Struct|BreakLinearColor _returnvalue)) (.G (Utilities|Struct|BreakLinearColor _returnvalue)) 1.0 (.A (Utilities|Struct|BreakLinearColor _returnvalue))) :!class /Script/Engine.MaterialInstanceDynamic))

(event EventStartPoison
  (bind _dynamic_material (Variables|Default|GetDynamic%20Material))
  (bind _returnvalue (Rendering|Material|GetVectorParameterValue _dynamic_material "TintValue" :!class /Script/Engine.MaterialInstanceDynamic))
  (Rendering|Material|SetVectorParameterValue _dynamic_material "TintValue" (Utilities|Struct|MakeLinearColor (.R (Utilities|Struct|BreakLinearColor _returnvalue)) 1.0 (.B (Utilities|Struct|BreakLinearColor _returnvalue)) (.A (Utilities|Struct|BreakLinearColor _returnvalue))) :!class /Script/Engine.MaterialInstanceDynamic))

(event EventStartHit
  (bind _dynamic_material (Variables|Default|GetDynamic%20Material))
  (bind _redvalue (Timeline|RedReduce PlayFromStart)
    (:Update
      (bind _returnvalue (Rendering|Material|GetVectorParameterValue _dynamic_material "TintValue" :!class /Script/Engine.MaterialInstanceDynamic))
      (Rendering|Material|SetVectorParameterValue _dynamic_material "TintValue" (Utilities|Struct|MakeLinearColor _redvalue (.G (Utilities|Struct|BreakLinearColor _returnvalue)) (.B (Utilities|Struct|BreakLinearColor _returnvalue)) (.A (Utilities|Struct|BreakLinearColor _returnvalue))) :!class /Script/Engine.MaterialInstanceDynamic))))

(event EventEndPoison
  (bind _dynamic_material (Variables|Default|GetDynamic%20Material))
  (bind _greenvalue (Timeline|GreenReduce PlayFromStart)
    (:Update
      (bind _returnvalue (Rendering|Material|GetVectorParameterValue _dynamic_material "TintValue" :!class /Script/Engine.MaterialInstanceDynamic))
      (Rendering|Material|SetVectorParameterValue _dynamic_material "TintValue" (Utilities|Struct|MakeLinearColor (.R (Utilities|Struct|BreakLinearColor _returnvalue)) _greenvalue (.B (Utilities|Struct|BreakLinearColor _returnvalue)) (.A (Utilities|Struct|BreakLinearColor _returnvalue))) :!class /Script/Engine.MaterialInstanceDynamic))))

(event EventEndFreeze
  (bind _dynamic_material (Variables|Default|GetDynamic%20Material))
  (Timeline|BlueReduce PlayFromStart
    (:Update
      (bind _returnvalue (Rendering|Material|GetVectorParameterValue _dynamic_material "TintValue" :!class /Script/Engine.MaterialInstanceDynamic))
      (Rendering|Material|SetVectorParameterValue _dynamic_material "TintValue" (Utilities|Struct|MakeLinearColor (.R (Utilities|Struct|BreakLinearColor _returnvalue)) (.G (Utilities|Struct|BreakLinearColor _returnvalue)) 0.0 (.A (Utilities|Struct|BreakLinearColor _returnvalue))) :!class /Script/Engine.MaterialInstanceDynamic))))

(event EventBeginPlay
  (bind _mesh (Variables|Character|GetMesh))
  (bind _returnvalue (Rendering|Material|CreateDynamicMaterialInstance _mesh 0 (Rendering|Material|GetMaterial _mesh 0) :!class /Script/Engine.PrimitiveComponent))
  (Variables|Default|SetDynamic%20Material _returnvalue)
  (Class|EnemyCharacter|FreezeAnimation)
  (Utilities|FlowControl|Delay (Math|Random|RandomFloatinRange 0.0 (/ 4.0 3.0)))
  (Class|EnemyCharacter|UnfreezeAnimation))

(event EventSpawnIndicator
  (params (_krfDamageAmount :type Float%20%28single-precision%29%20%28by%20ref%29))
  (bind _self self)
  (bind _returnvalue (Transformation|GetActorLocation _self))
  (bind _returnvalue_2 (UserInterface|CreateWidget "/Game/HUD/BP_HUDDamageIndicator.BP_HUDDamageIndicator_C"))
  (Rendering|Components|TextRender|SetText (Variables|/Game/HUD/BP_HUDDamageIndicator.BP_HUDDamageIndicator_C|GetDamageAmount _returnvalue_2) (Utilities|Text|ToText(Float) _krfDamageAmount "HalfToEven"))
  (UserInterface|Viewport|AddtoViewport _returnvalue_2 10)
  (Variables|/Game/HUD/BP_HUDDamageIndicator.BP_HUDDamageIndicator_C|SetLocation _returnvalue_2 _returnvalue)
  (Class|UserWidget|SetPositioninViewport _returnvalue_2 (.ScreenLocation (Class|PlayerController|ProjectWorldLocationtoScreen (Game|GetPlayerController 0) _returnvalue)) true))

(fn ConstructionScript)