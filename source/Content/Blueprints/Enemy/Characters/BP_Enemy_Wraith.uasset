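; Wraith enemy Blueprint that adds animation and ghost audio on top of a parent enemy class.
; BeginPlay flags the wraith anim Blueprint as moving, then calls the parent BeginPlay, which is skipped if that cast fails.
; ChangeState toggles the still-attack animation flag, on for Pre Attack and off for Idle or Seeking.
; Random rolls occasionally play a ghost noise on Seeking and a death sound when destroyed.
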(event EventBeginPlay
  (bind _asbp_wraith_anim_bluprint (Utilities|Casting|CastToBP_wraith_AnimBluprint (Components|SkeletalMesh|GetAnimInstance (Variables|Character|GetMesh))))
  (Variables|/Game/Animations/Enemies/Mobs/Flying/Wraith/BP_wraith_AnimBluprint.BP_wraith_AnimBluprint_C|Setis_moving _asbp_wraith_anim_bluprint true)
  (|CallParentFunction))

(event EventDestroyed
  (if (== (Math|Random|RandomIntegerinRange 0 6) 0)
    (Audio|PlaySoundatLocation "/Game/Sound/SoundWaves/Enemies/Ghost/Ghost_Death.Ghost_Death" (Transformation|GetActorLocation self))))

(fn ConstructionScript)

(fn ChangeState
  (params (New%20State :type EEnemyState%20Enum))
  (bind _asbp_wraith_anim_bluprint (Utilities|Casting|CastToBP_wraith_AnimBluprint (Components|SkeletalMesh|GetAnimInstance (Variables|Character|GetMesh))))
  (switch Utilities|FlowControl|Switch|SwitchonEEnemyState New%20State
    (:ENEMY_STATE_IDLE
      (Variables|/Game/Animations/Enemies/Mobs/Flying/Wraith/BP_wraith_AnimBluprint.BP_wraith_AnimBluprint_C|Setis_attacking_still _asbp_wraith_anim_bluprint false :!label _label))
    (:ENEMY_STATE_SEEKING
      (if (== (Math|Random|RandomIntegerinRange 0 8) 0)
        (Audio|PlaySoundatLocation "/Game/Sound/SoundCues/GhostNoise.GhostNoise" (Transformation|GetActorLocation))
        (goto _label)
        (else
          (goto _label))))
    (:ENEMY_STATE_PRE_ATTACK
      (Variables|/Game/Animations/Enemies/Mobs/Flying/Wraith/BP_wraith_AnimBluprint.BP_wraith_AnimBluprint_C|Setis_attacking_still _asbp_wraith_anim_bluprint true))))