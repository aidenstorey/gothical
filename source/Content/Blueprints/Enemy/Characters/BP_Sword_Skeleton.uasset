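; Sword skeleton enemy character that reacts to hits, drives its attack animations and leaves a physics version of itself when destroyed.
; The damage indicator event puts the melee AI controller into a timed hit state before calling the parent.
; State changes set the attack and hit flags on the skeleton's anim instance.
; On destruction it spawns the physics skeleton actor, lowered from the actor's location and matching the mesh's yaw.
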(event EventChangeState
  (params (NewState :type Byte :default 0))
  (bind _asbp_sword_skeleton_anim (Utilities|Casting|CastToBP_SwordSkeleton_Anim (Components|SkeletalMesh|GetAnimInstance (Variables|Character|GetMesh))))
  (switch Utilities|FlowControl|Switch|SwitchonEEnemyState NewState
    (:ENEMY_STATE_PRE_ATTACK
      (Variables|/Game/Animations/Enemies/Mobs/Melee/SwordSkeleton/BP_SwordSkeleton_Anim.BP_SwordSkeleton_Anim_C|SetIsAttacking _asbp_sword_skeleton_anim true)
      (Variables|/Game/Animations/Enemies/Mobs/Melee/SwordSkeleton/BP_SwordSkeleton_Anim.BP_SwordSkeleton_Anim_C|SetIsHit _asbp_sword_skeleton_anim false :!label _label))
    (:ENEMY_STATE_POST_ATTACK
      (Variables|/Game/Animations/Enemies/Mobs/Melee/SwordSkeleton/BP_SwordSkeleton_Anim.BP_SwordSkeleton_Anim_C|SetIsAttacking _asbp_sword_skeleton_anim false)
      (goto _label))
    (:ENEMY_STATE_PRE_HIT
      (Variables|/Game/Animations/Enemies/Mobs/Melee/SwordSkeleton/BP_SwordSkeleton_Anim.BP_SwordSkeleton_Anim_C|SetIsHit _asbp_sword_skeleton_anim true))
    (:ENEMY_STATE_POST_HIT
      (Variables|/Game/Animations/Enemies/Mobs/Melee/SwordSkeleton/BP_SwordSkeleton_Anim.BP_SwordSkeleton_Anim_C|SetIsHit _asbp_sword_skeleton_anim false))))

(event EventDestroyed
  (Game|SpawnActorfromClass "/Game/Blueprints/Enemy/Characters/BP_Sword_Skeleton_Physics.BP_Sword_Skeleton_Physics_C" (Math|Transform|MakeTransform (- (Transformation|GetActorLocation) "0, 0,90.000000") (Class|KismetMathLibrary|MakeRot 0.0 (.Yaw (Class|KismetMathLibrary|BreakRot (Transformation|GetWorldRotation (Variables|Character|GetMesh)))) 0.0) "1,1,1") false 0 0))

(event EventSpawnIndicator
  (params (_krfDamageAmount :type Float%20%28single-precision%29%20%28by%20ref%29))
  (bind _returnvalue (AI|GetAIController self))
  (bind _asbp_enemy_controller_melee (Utilities|Casting|CastToBP_Enemy_Controller_Melee _returnvalue))
  (Class|EnemyControllerBase|EnterHitState _asbp_enemy_controller_melee 1.17)
  (|CallParentFunction _krfDamageAmount))

(fn ConstructionScript
  (|CallParentFunction))