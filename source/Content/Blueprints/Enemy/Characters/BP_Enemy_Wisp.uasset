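; Wisp enemy Blueprint that adds wisp-specific particle effects to behavior inherited from its parent class.
; The SpawnIndicator event spawns a hit emitter at the actor's location, then passes the damage amount on to the parent's damage indicator.
; ChangeState spawns an explosion emitter at the same location when the new state is Post Explode, with no parent call and no handling for other states.
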(event EventSpawnIndicator
  (params (_krfDamageAmount :type Float%20%28single-precision%29%20%28by%20ref%29))
  (Effects|SpawnEmitteratLocation 0 "/Game/VFX/P_WispHit.P_WispHit" (Transformation|GetActorLocation self))
  (|CallParentFunction _krfDamageAmount))

(fn ConstructionScript
  (|CallParentFunction))

(fn ChangeState
  (params (NewState :type EEnemyState%20Enum))
  (switch Utilities|FlowControl|Switch|SwitchonEEnemyState NewState
    (:ENEMY_STATE_POST_EXPLODE
      (Effects|SpawnEmitteratLocation 0 "/Game/VFX/P_WispExplode.P_WispExplode" (Transformation|GetActorLocation self)))))