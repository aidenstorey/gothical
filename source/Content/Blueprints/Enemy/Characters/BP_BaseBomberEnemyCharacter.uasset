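; Base character Blueprint for bomber enemies, whose only logic here displays a damage number on screen at the enemy's position.
; SpawnIndicator creates a BP_HUDDamageIndicator widget, sets its text from the damage amount and adds it to the viewport.
; It passes the actor's world location to the widget and sets its initial position by projecting that location through the first player controller.
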(event EventSpawnIndicator
  (params (_krfDamageAmount :type Float%20%28single-precision%29%20%28by%20ref%29))
  (bind _self self)
  (bind _returnvalue (Transformation|GetActorLocation _self))
  (bind _returnvalue_2 (UserInterface|CreateWidget "/Game/HUD/BP_HUDDamageIndicator.BP_HUDDamageIndicator_C"))
  (Rendering|Components|TextRender|SetText (Variables|/Game/HUD/BP_HUDDamageIndicator.BP_HUDDamageIndicator_C|GetDamageAmount _returnvalue_2) (Utilities|Text|ToText(Float) _krfDamageAmount "HalfToEven"))
  (UserInterface|Viewport|AddtoViewport _returnvalue_2 10)
  (Variables|/Game/HUD/BP_HUDDamageIndicator.BP_HUDDamageIndicator_C|SetLocation _returnvalue_2 _returnvalue)
  (Class|UserWidget|SetPositioninViewport _returnvalue_2 (.ScreenLocation (Class|PlayerController|ProjectWorldLocationtoScreen (Game|GetPlayerController 0) _returnvalue)) true))

(fn ConstructionScript)