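; BP_Enemy_Melee_spawner is a damageable actor that releases BP_Skeleton_Physics actors when destroyed.
; Each hit shows a floating damage-number widget at its projected screen position and subtracts from Health, destroying the actor at zero.
; The Destroyed event runs a short loop that spawns skeletons at the actor's transform, ignoring collision, and triggers a strong camera shake on each iteration.
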(event Game|Damage|EventAnyDamage
  (params (Damage :type Float%20%28single-precision%29) (DamageType :type Damage%20Type%20Object%20Reference) (InstigatedBy :type Controller%20Object%20Reference) (DamageCauser :type Actor%20Object%20Reference))
  (bind _self self)
  (bind _returnvalue (Transformation|GetActorLocation _self))
  (bind _returnvalue_2 (UserInterface|CreateWidget "/Game/HUD/BP_HUDDamageIndicator.BP_HUDDamageIndicator_C"))
  (Rendering|Components|TextRender|SetText (Variables|/Game/HUD/BP_HUDDamageIndicator.BP_HUDDamageIndicator_C|GetDamageAmount _returnvalue_2) (Utilities|Text|ToText(Float) Damage "HalfToEven"))
  (UserInterface|Viewport|AddtoViewport _returnvalue_2 10)
  (Variables|/Game/HUD/BP_HUDDamageIndicator.BP_HUDDamageIndicator_C|SetLocation _returnvalue_2 _returnvalue)
  (Class|UserWidget|SetPositioninViewport _returnvalue_2 (.ScreenLocation (Class|PlayerController|ProjectWorldLocationtoScreen (Game|GetPlayerController 0) _returnvalue)) true)
  (bind _output_get (Variables|Default|SetHealth (- (Variables|Default|GetHealth) Damage)))
  (if (<= _output_get 0.0)
    (Actor|DestroyActor)))

(event EventDestroyed
  (for _index (range 0 2)
    (Game|SpawnActorfromClass "/Game/Blueprints/Enemy/Characters/BP_Skeleton_Physics.BP_Skeleton_Physics_C" (Transformation|GetActorTransform) true 0 0)
    (Class|PlayerController|ClientPlayCameraShake (Game|GetPlayerController 0) "/Game/Blueprints/BP_Camera_Shake.BP_Camera_Shake_C" 1e+01 "CameraLocal" "0, 0, 0")))

(fn ConstructionScript)